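; Game mode that provides functions for spawning healing and damaging actors at randomly chosen placed markers.
; SpawnActionHeal and SpawnActionDamage each gather their marker class, then loop to spawn at a random marker's transform, removing and destroying it so no spot repeats.
; SpawnNewActor separately spawns a damaging actor at the world origin.
; BeginPlay and Tick are empty, and nothing here calls these functions.
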(event EventBeginPlay)

(event EventTick
  (params (DeltaSeconds :type Float%20%28single-precision%29)))

(fn ConstructionScript)

(fn SpawnNewActor
  (Game|SpawnActorfromClass "/Game/Blueprints/BP_DamagingActor.BP_DamagingActor_C" (Math|Transform|MakeTransform "0, 0, 0") "Undefined" "MultiplyWithRoot" 0 0))

(fn SpawnActionHeal
  (bind _outactors (Actor|GetAllActorsOfClass "/Game/Blueprints/Spawn_Healing_Actor.Spawn_Healing_Actor_C"))
  (LocalVariables|SetHealLocalSpawnReferences _outactors)
  (for _index (range 0 1)
    (LocalVariables|SetHealLocalItem (.OutItem (Utilities|Array|Random (LocalVariables|GetHealLocalSpawnReferences))))
    (Game|SpawnActorfromClass "/Game/Blueprints/BP_HealingActor.BP_HealingActor_C" (Math|Transform|MakeTransform (Transformation|GetActorLocation (LocalVariables|GetHealLocalItem)) (Transformation|GetActorRotation (LocalVariables|GetHealLocalItem))) "Undefined" "MultiplyWithRoot" 0 0)
    (Utilities|Array|RemoveItem (LocalVariables|GetHealLocalSpawnReferences) (LocalVariables|GetHealLocalItem))
    (Actor|DestroyActor (LocalVariables|GetHealLocalItem))))

(fn SpawnActionDamage
  (bind _outactors (Actor|GetAllActorsOfClass "/Game/Blueprints/Spawn_Damaging_Actor.Spawn_Damaging_Actor_C"))
  (LocalVariables|SetLocalSpawnReferences _outactors)
  (for _index (range 0 1)
    (LocalVariables|SetLocalItem (.OutItem (Utilities|Array|Random (LocalVariables|GetLocalSpawnReferences))))
    (Game|SpawnActorfromClass "/Game/Blueprints/BP_DamagingActor.BP_DamagingActor_C" (Math|Transform|MakeTransform (Transformation|GetActorLocation (LocalVariables|GetLocalItem)) (Transformation|GetActorRotation (LocalVariables|GetLocalItem))) "Undefined" "MultiplyWithRoot" 0 0)
    (Utilities|Array|RemoveItem (LocalVariables|GetLocalSpawnReferences) (LocalVariables|GetLocalItem))
    (Actor|DestroyActor (LocalVariables|GetLocalItem))))