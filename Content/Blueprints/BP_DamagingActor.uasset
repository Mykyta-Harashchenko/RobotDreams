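; BP_DamagingActor is a moving hazard that damages any actor overlapping its capsule.
; Each Tick it turns in yaw by RotateSpeed and advances along the new forward vector by MoveSpeed, both scaled by delta time, using a swept move.
; Capsule overlap applies fixed damage to the other actor and prints a debug string, with no filtering of what was hit.
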(event OnComponentBeginOverlap(Capsule)
  (params (OverlappedComponent :type Primitive%20Component%20Object%20Reference) (OtherActor :type Actor%20Object%20Reference) (OtherComp :type Primitive%20Component%20Object%20Reference) (OtherBodyIndex :type Integer) (bFromSweep :type Boolean) (SweepResult :type Hit%20Result%20Structure%20%28by%20ref%29))
  (Development|PrintString "collsiiso")
  (Game|Damage|ApplyDamage OtherActor 25.0 0 0))

(event EventBeginPlay)

(event Collision|EventActorBeginOverlap
  (params (OtherActor :type Actor%20Object%20Reference)))

(event EventTick
  (params (DeltaSeconds :type Float%20%28single-precision%29))
  (bind _returnvalue (Transformation|GetActorRotation))
  (bind _rotatespeed (Variables|Default|GetRotateSpeed))
  (bind (_roll _pitch _yaw) (Math|Rotator|BreakRotator _returnvalue))
  (bind _returnvalue_2 (* DeltaSeconds _rotatespeed))
  (bind _returnvalue_3 (+ _yaw _returnvalue_2))
  (bind _returnvalue_4 (Math|Rotator|MakeRotator _roll _pitch _returnvalue_3))
  (Transformation|SetActorLocationAndRotation (+ (* (Math|Vector|GetForwardVector _returnvalue_4) (* DeltaSeconds (Variables|Default|GetMoveSpeed))) (Transformation|GetActorLocation)) _returnvalue_4 true))

(fn ConstructionScript)